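; Checkpoint actor that records a respawn position when the third-person character enters it.
; An overlap on CheckpointCollision filters for BP_ThirdPersonCharacter, then calls SelectCheckpoint.
; SelectCheckpoint writes the RespawnLocation component's world location to LastCheckpointCoords on BP_GameInstance and prints it.
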(event `self.CheckpointCollision.OnComponentBeginOverlap`
  (params (OverlappedComponent :type "PrimitiveComponent Object Reference") (OtherActor :type "Actor Object Reference") (OtherComp :type "PrimitiveComponent Object Reference") (OtherBodyIndex :type Integer) (bFromSweep :type Boolean) (SweepResult :type "HitResult Structure (by ref)"))
  (cast `/Game/ThirdPerson/Blueprints/BP_ThirdPersonCharacter` OtherActor)
  (`self.SelectCheckpoint`))

(fn `SelectCheckpoint`
  (bind _asbp_game_instance (cast `/Game/Blueprints/BP_GameInstance` (`GameplayStatics.GetGameInstance`)))
  (bind _output_get (set `/Game/Blueprints/BP_GameInstance.LastCheckpointCoords` (`SceneComponent.K2_GetComponentLocation` (`self.RespawnLocation`)) _asbp_game_instance))
  (`KismetSystemLibrary.PrintString` (`KismetStringLibrary.Concat_StrStr` "Last checkpoint at " (`KismetStringLibrary.Conv_VectorToString` _output_get))))

(fn `UserConstructionScript`)